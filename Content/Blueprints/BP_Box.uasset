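; BP_Box is a grabbable box that attaches to a hand socket with collision off and can snap onto another interactable when released.
; On release, a Detect macro box-traces toward six end points for BPI_Interactuable actors, then teleports the box to the drop point paired with their nearest distance point.
; It exposes its own six point pairs through GetDistanceAndDropPoints.
; Occupied-slot tracking (LocationsUsed) is initialized but unwired.
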(event `self.ReceiveBeginPlay`
  (set `self.DropPositionsArray` (`|MakeArray` (`self.DropPosition1`) (`self.DropPosition2`) (`self.DropPosition3`) (`self.DropPosition4`) (`self.DropPosition5`) (`self.DropPosition6`)))
  (set `self.endDetectionsArray` (`|MakeArray` (`self.EndDetection1`) (`self.EndDetection2`) (`self.EndDetection3`) (`self.EndDetection4`) (`self.EndDetection5`) (`self.EndDetection6`)))
  (set `self.DistancePointsArray` (`|MakeArray` (`self.DistancePoint1`) (`self.DistancePoint2`) (`self.DistancePoint3`) (`self.DistancePoint4`) (`self.DistancePoint5`) (`self.DistancePoint6`)))
  (set `self.LocationsUsed` (`|MakeArray` false false false false false false)))

(event `/Game/Blueprints/BPI_Interactuable.EndInteraction`
  (params (Location :type "Vector Structure") (Rotation :type "Rotator Structure"))
  (set `self.grabbed` false)
  (`self.K2_DetachFromActor` self "KeepWorld" "KeepWorld" "KeepWorld")
  (`SceneComponent.K2_SetWorldLocationAndRotation` (`self.RootComponent`) Location Rotation false true)
  (`KismetSystemLibrary.DelayUntilNextTick`)
  (bind (_array_index _distancepoints _droppoints _asbpi_interactuable) (`self.Detect`)
    (:`NewParam2`
      (`/Engine/EditorBlueprintResources/StandardMacros.IsValid` (`KismetSystemLibrary.Conv_InterfaceToObject` _asbpi_interactuable)
        (:`Is Valid`
          (for (_array_element _array_index_2) _distancepoints
            (bind _returnvalue (`KismetMathLibrary.Vector_Distance` (`SceneComponent.K2_GetComponentLocation` _array_element) (`SceneComponent.K2_GetComponentLocation` (`self.SM_ChamferCube`))))
            (if (< _returnvalue (`self.lessDistance`))
              (set `self.lessDistance` _returnvalue)
              (set `self.LessDistanceIndex` _array_index_2)))
          (bind _output (`|GetArrayItem` _droppoints (`self.LessDistanceIndex`)))
          (`SceneComponent.K2_SetWorldLocationAndRotation` (`self.ParentSphere`) (`SceneComponent.K2_GetComponentLocation` _output) (`SceneComponent.K2_GetComponentRotation` _output) false true)
          (`PrimitiveComponent.SetCollisionEnabled` (`self.SM_ChamferCube`) "QueryAndPhysics")
          (`PrimitiveComponent.SetCollisionEnabled` (`self.Box`) "QueryAndPhysics")
          (set `self.lessDistance` 1000000000000000.0)
          (set `self.LessDistanceIndex` 0))))
    (:`Completed`
      (`PrimitiveComponent.SetCollisionEnabled` (`self.SM_ChamferCube`) "QueryAndPhysics")
      (`PrimitiveComponent.SetCollisionEnabled` (`self.Box`) "QueryAndPhysics"))))

(fn `GetDistanceAndDropPoints`
  (returns (DistancePoints :type "Array of SceneComponent Object Reference") (DropPoints :type "Array of SceneComponent Object Reference"))
  (return (`self.DistancePointsArray`) (`self.DropPositionsArray`)))

(fn `Interact`
  (params (Component :type "/Game/Characters/Racer/BP_Maincharacter Object Reference"))
  (returns (typeOfObject :type "/Game/Blueprints/E_TypeOfObject Enum"))
  (if (not (`self.grabbed`))
    (set `self.grabbed` true)
    (`KismetSystemLibrary.PrintString` "Hello")
    (`PrimitiveComponent.SetCollisionEnabled` (`self.SM_ChamferCube`) "NoCollision")
    (`PrimitiveComponent.SetCollisionEnabled` (`self.Box`) "NoCollision")
    (`self.K2_AttachToComponent` self (`/Game/Characters/Racer/BP_Maincharacter.HandSocket` Component) "None" "SnapToTarget" "SnapToTarget" "KeepWorld" true)
    (return (`self.typeOfObject`))))

(fn `UserConstructionScript`)