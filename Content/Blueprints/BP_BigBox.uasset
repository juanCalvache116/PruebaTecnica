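; BP_BigBox is an interactable box that a player can move back and forth along a fixed track.
; Interact snaps and attaches the player to the nearer of two Direction points, which also sets the travel sign.
; While the player's MovePull is active, Tick advances a clamped Alpha that lerps the Cube between InitialPosition and FinalPosition.
; EndInteraction detaches the player and stops the movement.
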(event `self.ReceiveBeginPlay`)

(event `self.ReceiveTick`
  (params (DeltaSeconds :type "Float (single-precision)"))
  (bind _snapedplayer (`self.SnapedPlayer`))
  (set `self.Delta Seconds` DeltaSeconds)
  (`/Engine/EditorBlueprintResources/StandardMacros.IsValid` _snapedplayer
    (:`Is Valid`
      (if (and (`self.beingPulled`) (`/Game/Characters/Racer/BP_Maincharacter.movePull` _snapedplayer))
        (set `self.Alpha` (`KismetMathLibrary.MapRangeClamped` (+ (* (`self.Delta Seconds`) 0.1 (`KismetMathLibrary.SelectFloat` -1.0 1.0 (`self.direction1/2`))) (`self.Alpha`)) 0.0 1.0 0.0 1.0))
        (`SceneComponent.K2_SetWorldLocation` (`self.Cube`) (`KismetMathLibrary.VLerp` (`SceneComponent.K2_GetComponentLocation` (`self.InitialPosition`)) (`SceneComponent.K2_GetComponentLocation` (`self.FinalPosition`)) (`self.Alpha`)) false false)))))

(event `/Game/Blueprints/BPI_Interactuable.EndInteraction`
  (params (Location :type "Vector Structure") (Rotation :type "Rotator Structure"))
  (`SceneComponent.K2_DetachFromComponent` (`Actor.RootComponent` (`self.SnapedPlayer`)) "KeepWorld" "KeepWorld" "KeepWorld" true)
  (set `self.beingPulled` false)
  (set `self.SnapedPlayer` null))

(fn `Interact`
  (params (Component :type "/Game/Characters/Racer/BP_Maincharacter Object Reference"))
  (returns (typeOfObject :type "/Game/Blueprints/E_TypeOfObject Enum"))
  (bind _output_get (set `self.SnapedPlayer` Component))
  (bind _returnvalue (`SceneComponent.K2_GetComponentLocation` (`Actor.RootComponent` _output_get)))
  (set `self.direction1/2` (> (`KismetMathLibrary.Vector_Distance` _returnvalue (`SceneComponent.K2_GetComponentLocation` (`self.Direction1`))) (`KismetMathLibrary.Vector_Distance` _returnvalue (`SceneComponent.K2_GetComponentLocation` (`self.Direction2`)))))
  (`self.K2_AttachToComponent` _output_get (select `bool` (`self.direction1/2`) :`false` (`self.Direction1`) :`true` (`self.Direction2`)) "None" "SnapToTarget" "SnapToTarget" "KeepWorld" true)
  (set `self.beingPulled` true)
  (return "NewEnumerator1"))

(fn `UserConstructionScript`)